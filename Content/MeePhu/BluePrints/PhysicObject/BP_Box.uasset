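; BP_Box is a grabbable, destructible physics box for VR, with a PhysicsConstraint joining its CollisionBox and Cube.
; While held through GrabComponent, the Cube ignores the PhysicsBody channel so it does not collide with the hand, and blocks it again when dropped.
; Damage lowers HP, gated by a DoOnce with a one-second cooldown and a Physic_VRPawn player check, and destroys the actor at zero.
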(event `self.ReceiveBeginPlay`
  (`PhysicsConstraintComponent.SetConstrainedComponents` (`self.PhysicsConstraint`) (`self.CollisionBox`) "None" (`self.Cube`) "None")
  (`KismetSystemLibrary.PrintString` (`KismetStringLibrary.Conv_DoubleToString` (`self.HP`))))

(event `self.ReceiveAnyDamage`
  (params (Damage :type "Float (single-precision)") (DamageType :type "DamageType Object Reference") (InstigatedBy :type "Controller Object Reference") (DamageCauser :type "Actor Object Reference"))
  (cast `/Game/MeePhu/BluePrints/Physic_VRPawn` (`GameplayStatics.GetPlayerCharacter` 0))
  (`/Engine/EditorBlueprintResources/StandardMacros.DoOnce` false :!label _label
    (:`Completed`
      (bind _output_get (set `self.HP` (- (`self.HP`) Damage)))
      (`KismetSystemLibrary.PrintString` (`KismetStringLibrary.Conv_DoubleToString` _output_get))
      (if (<= (`self.HP`) 0.0)
        (`self.K2_DestroyActor`)
        (else
          (`KismetSystemLibrary.Delay` 1.0)
          (goto _label :!via `Reset`))))))

(event `self.GrabComponent.OnGrabbed`
  ;[0.3369 1 0.2919] No need to let the object touch the hand while the hand is holding the object.
  (`PrimitiveComponent.SetCollisionResponseToChannel` (`self.Cube`) "ECC_PhysicsBody" "ECR_Ignore"))

(event `self.GrabComponent.OnDropped`
  ;[0.3369 1 0.2919] No need to let the object touch the hand while the hand is holding the object.
  (`PrimitiveComponent.SetCollisionResponseToChannel` (`self.Cube`) "ECC_PhysicsBody" "ECR_Block"))

(fn `UserConstructionScript`)